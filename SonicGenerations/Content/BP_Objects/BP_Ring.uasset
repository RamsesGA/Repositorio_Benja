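; Collectible ring pickup that grants rings and score when the Sonic character's capsule overlaps its hitbox, then plays a particle and sound and destroys itself.
; By default it uses a RotatingMovement component.
; EnableRingPhysics switches it to a simulated physics body, stops the rotation and can start a timer that calls DestroyRing for a particle-only removal.
; In physics mode, sufficiently fast impacts can play a collision sound.
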(event OnComponentBeginOverlap(RingHitbox)
  (params (OverlappedComponent :type Primitive%20Component%20Object%20Reference) (OtherActor :type Actor%20Object%20Reference) (OtherComp :type Primitive%20Component%20Object%20Reference) (OtherBodyIndex :type Integer) (bFromSweep :type Boolean) (SweepResult :type Hit%20Result%20Structure%20%28by%20ref%29))
  (bind _ring (Variables|Default|GetRing))
  (bind _returnvalue (Transformation|GetWorldLocation _ring))
  ;[1 1 1] Ring Physics
  (bind _asbp_sonic_fbx (Utilities|Casting|CastToBP_SonicFBX OtherActor))
  (if (== (Variables|/Script/Engine.Character|GetCapsuleComponent _asbp_sonic_fbx) OtherComp)
    (Default|GiveRings _asbp_sonic_fbx (Variables|Default|GetRingValue) false)
    (Default|AddScores _asbp_sonic_fbx (Variables|Default|GetScoreValue))
    (Effects|SpawnEmitteratLocation (Variables|Default|GetRingParticle) _returnvalue)
    (Audio|PlaySoundatLocation (Variables|Default|GetRingSound) _returnvalue "0, 0, 0" 1.0 1.0 0.0 0 0 0)
    (Actor|DestroyActor)))

(event Collision|EventHit
  (params (MyComp :type Primitive%20Component%20Object%20Reference) (Other :type Actor%20Object%20Reference) (OtherComp :type Primitive%20Component%20Object%20Reference) (bSelfMoved :type Boolean) (HitLocation :type Vector :default "0, 0, 0") (HitNormal :type Vector :default "0, 0, 0") (NormalImpulse :type Vector :default "0, 0, 0") (Hit :type Hit%20Result%20Structure%20%28by%20ref%29))
  (if (Variables|Default|GetPlayImpactSound)
    (if (>= (Math|Vector|VectorLength (Transformation|GetVelocity)) 4e+02)
      (if (Variables|Default|GetPhysicsEnabled)
        (Audio|PlaySoundatLocation (Variables|Default|GetCollisionSound) (Transformation|GetWorldLocation (Variables|Default|GetRing)) "0, 0, 0" 1.0 1.0 0.0 0 0 0)))))

(fn ConstructionScript)

(fn DestroyRing
  (Effects|SpawnEmitteratLocation (Variables|Default|GetRingParticle) (Transformation|GetActorLocation))
  (Actor|DestroyActor))

(fn EnableRingPhysics
  (params (DestroyAfterTimer :type Boolean) (Timer :type Float%20%28single-precision%29))
  (bind _ring (Variables|Default|GetRing))
  (Physics|SetSimulatePhysics _ring true)
  (Variables|Default|SetPhysicsEnabled true)
  (Collision|SetCollisionEnabled _ring "QueryAndPhysics")
  (Components|Activation|Deactivate (Variables|Default|GetRotatingMovement))
  (if DestroyAfterTimer
    (Utilities|Time|SetTimerbyFunctionName 0 "DestroyRing" Timer)))